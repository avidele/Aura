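; Behavior tree service that flags whether the target actor counts as reachable by the controlled pawn, judged purely by proximity.
; On activation only, with no tick update, it takes the largest absolute axis offset between the pawn and the blackboard target actor.
; It sets the reachable blackboard bool by comparing that offset to a fixed threshold, a box-shaped range check without any navigation query.
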(event `self.ReceiveActivationAI`
  (params (OwnerController :type "AIController Object Reference") (ControlledPawn :type "Pawn Object Reference"))
  (if (< (`KismetMathLibrary.GetMaxElement` (`KismetMathLibrary.Vector_GetAbs` (- (`Actor.K2_GetActorLocation` ControlledPawn) (`Actor.K2_GetActorLocation` (`BTFunctionLibrary.GetBlackboardValueAsActor` (`self.TargetActor`)))))) 500.0)
    (`BTFunctionLibrary.SetBlackboardValueAsBool` (`self.bReachable`) true)
    (else
      (`BTFunctionLibrary.SetBlackboardValueAsBool` (`self.bReachable`)))))