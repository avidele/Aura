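; AIC_Enemy is an enemy AI controller that runs BT_Enemy and tracks the player through AI perception.
; When it senses an actor tagged Player, it writes the TargetActor and HasLineOfSight blackboard keys and cancels any pending lost-sight timer.
; When sensing fails, it clears line of sight at once but keeps the target until a short timer expires, then empties TargetActor.
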(event `self.ReceiveBeginPlay`
  (`self.RunBehaviorTree` "/Game/Blueprints/AI/BT_Enemy.BT_Enemy"))

(event `self.AIPerception.OnTargetPerceptionUpdated`
  (params (Actor :type "Actor Object Reference") (Stimulus :type "AIStimulus Structure"))
  (set `self.PerceivedActor` Actor)
  (if (`self.ActorHasTag` Actor "Player")
    (if (`.bSuccessfullySensed` (break `AIStimulus` Stimulus))
      (`KismetSystemLibrary.K2_ClearAndInvalidateTimerHandle` (`self.LostSightTimer`))
      (`self.UpdateTargetKey` (`self.PerceivedActor`))
      (`self.UpdateSightKey` true)
      (else
        (bind _returnvalue (`KismetSystemLibrary.K2_SetTimerDelegate` (delegate `LostSight`) 4.0))
        (set `self.LostSightTimer` _returnvalue)
        (`self.UpdateSightKey` false)))))

(event `LostSight`
  (`self.UpdateTargetKey` null))

(fn `UpdateSightKey`
  (params (HasLineOfSight :type Boolean))
  (`BlackboardComponent.SetValueAsBool` (`self.Blackboard`) "HasLineOfSight" HasLineOfSight))

(fn `UpdateTargetKey`
  (params (TargetActor :type "Actor Object Reference"))
  (`BlackboardComponent.SetValueAsObject` (`self.Blackboard`) "TargetActor" TargetActor))

(fn `UserConstructionScript`)